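; BP_Notepad is an interactable notepad that shows its Texts in a W_Note widget for five seconds.
; Character overlap with its Sphere calls ObjectiveChanger, then shows the note only if the controller is moving to this notepad, clearing that flag.
; PlayerOverlapCheck covers a player already inside the Sphere, jumping straight to the note display without the objective call or target check.
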(event OnComponentBeginOverlap(Sphere)
  (params (OverlappedComponent :type Primitive%20Component%20Object%20Reference) (OtherActor :type Actor%20Object%20Reference) (OtherComp :type Primitive%20Component%20Object%20Reference) (OtherBodyIndex :type Integer) (bFromSweep :type Boolean) (SweepResult :type Hit%20Result%20Structure%20%28by%20ref%29))
  (bind _astop_down_character (Utilities|Casting|CastToTopDownCharacter OtherActor))
  (Variables|Default|SetTopDownCharacter _astop_down_character)
  (Default|ObjectiveChanger (Variables|Default|GetTopDownCharacter) 1)
  (if (and (Variables|/Game/TopDownBP/Blueprints/TopDownController.TopDownController_C|GetMovingToInteractable (.AsTop%20Down%20Controller (Utilities|Casting|CastToTopDownController (Pawn|GetController (Variables|Default|GetTopDownCharacter))))) (== (Variables|/Game/TopDownBP/Blueprints/TopDownController.TopDownController_C|GetInteractable (.AsTop%20Down%20Controller (Utilities|Casting|CastToTopDownController (Pawn|GetController (Variables|Default|GetTopDownCharacter))))) self))
    (Variables|/Game/TopDownBP/Blueprints/TopDownController.TopDownController_C|SetMovingToInteractable (.AsTop%20Down%20Controller (Utilities|Casting|CastToTopDownController (Pawn|GetController (Variables|Default|GetTopDownCharacter)))) false)
    (bind _returnvalue (UserInterface|CreateWidget "/Game/UI/Widgets/W_Note.W_Note_C" 0 (Variables|Default|GetTexts)))
    (bind _output_get (Variables|/Game/TopDownBP/Blueprints/TopDownCharacter.TopDownCharacter_C|SetwidgeRef (Variables|Default|GetTopDownCharacter) _returnvalue))
    (UserInterface|Viewport|AddtoViewport _returnvalue 0)
    (Utilities|FlowControl|Delay 5.0)
    (Widget|RemovefromParent _output_get)))

(event Custom|PlayerOverlapCheck
  (bind _sphere (Variables|Default|GetSphere))
  (bind _overlappingactors (Collision|GetOverlappingActors _sphere "/Game/TopDownBP/Blueprints/TopDownCharacter.TopDownCharacter_C" :!class /Script/Engine.PrimitiveComponent))
  (if (Utilities|Array|ContainsItem _overlappingactors (Game|Player|GetPlayerPawn 0))
    (Variables|Default|SetTopDownCharacter (.AsTop%20Down%20Character (Utilities|Casting|CastToTopDownCharacter (Utilities|Array|Get(acopy) _overlappingactors))))
    (Variables|/Game/TopDownBP/Blueprints/TopDownController.TopDownController_C|SetMovingToInteractable (.AsTop%20Down%20Controller (Utilities|Casting|CastToTopDownController (Pawn|GetController (Variables|Default|GetTopDownCharacter)))) false)
    (bind _returnvalue (UserInterface|CreateWidget "/Game/UI/Widgets/W_Note.W_Note_C" 0 (Variables|Default|GetTexts)))
    (bind _output_get (Variables|/Game/TopDownBP/Blueprints/TopDownCharacter.TopDownCharacter_C|SetwidgeRef (Variables|Default|GetTopDownCharacter) _returnvalue))
    (UserInterface|Viewport|AddtoViewport _returnvalue 0)
    (Utilities|FlowControl|Delay 5.0)
    (Widget|RemovefromParent _output_get)))

(event EventBeginPlay)

(event Collision|EventActorBeginOverlap
  (params (OtherActor :type Actor%20Object%20Reference)))

(event EventTick
  (params (DeltaSeconds :type Float%20%28single-precision%29)))

(fn ConstructionScript)