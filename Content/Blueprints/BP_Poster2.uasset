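; BP_Poster2 is an interactable poster that opens a W_Poster2 widget for the top-down player character.
; It opens when the character enters its Sphere while moving to this poster, or when PlayerOverlapCheck finds the player already inside.
; Both paths clear the controller's MovingToInteractable flag, then use the character's ViewportFull flag to avoid stacking widgets, storing the new widget in WidgeRef.
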(event OnComponentBeginOverlap(Sphere)
  (params (OverlappedComponent :type Primitive%20Component%20Object%20Reference) (OtherActor :type Actor%20Object%20Reference) (OtherComp :type Primitive%20Component%20Object%20Reference) (OtherBodyIndex :type Integer) (bFromSweep :type Boolean) (SweepResult :type Hit%20Result%20Structure%20%28by%20ref%29))
  (bind _astop_down_character (Utilities|Casting|CastToTopDownCharacter OtherActor))
  (Variables|Default|SetTop%20Down%20Character _astop_down_character)
  (if (and (Variables|/Game/TopDownBP/Blueprints/TopDownController.TopDownController_C|GetMovingToInteractable (.AsTop%20Down%20Controller (Utilities|Casting|CastToTopDownController (Pawn|GetController (Variables|Default|GetTop%20Down%20Character))))) (== (Variables|/Game/TopDownBP/Blueprints/TopDownController.TopDownController_C|GetInteractable (.AsTop%20Down%20Controller (Utilities|Casting|CastToTopDownController (Pawn|GetController (Variables|Default|GetTop%20Down%20Character))))) self))
    (Variables|/Game/TopDownBP/Blueprints/TopDownController.TopDownController_C|SetMovingToInteractable (.AsTop%20Down%20Controller (Utilities|Casting|CastToTopDownController (Pawn|GetController (Variables|Default|GetTop%20Down%20Character)))) false)
    (if (not (Variables|/Game/TopDownBP/Blueprints/TopDownCharacter.TopDownCharacter_C|GetviewportFull (Variables|Default|GetTop%20Down%20Character)))
      (bind _returnvalue (UserInterface|CreateWidget "/Game/UI/Widgets/W_Poster2.W_Poster2_C" 0 self))
      (Variables|/Game/TopDownBP/Blueprints/TopDownCharacter.TopDownCharacter_C|SetwidgeRef (Variables|Default|GetTop%20Down%20Character) _returnvalue)
      (UserInterface|Viewport|AddtoViewport _returnvalue 0)
      (Variables|/Game/TopDownBP/Blueprints/TopDownCharacter.TopDownCharacter_C|SetviewportFull (Variables|Default|GetTop%20Down%20Character) true))))

(event Custom|PlayerOverlapCheck
  (bind _sphere (Variables|Default|GetSphere))
  (bind _overlappingactors (Collision|GetOverlappingActors _sphere "/Game/TopDownBP/Blueprints/TopDownCharacter.TopDownCharacter_C" :!class /Script/Engine.PrimitiveComponent))
  (if (Utilities|Array|ContainsItem _overlappingactors (Game|Player|GetPlayerPawn 0))
    (Variables|Default|SetTop%20Down%20Character (.AsTop%20Down%20Character (Utilities|Casting|CastToTopDownCharacter (Utilities|Array|Get(acopy) _overlappingactors))))
    (Variables|/Game/TopDownBP/Blueprints/TopDownController.TopDownController_C|SetMovingToInteractable (.AsTop%20Down%20Controller (Utilities|Casting|CastToTopDownController (Pawn|GetController (Variables|Default|GetTop%20Down%20Character)))) false)
    (if (not (Variables|/Game/TopDownBP/Blueprints/TopDownCharacter.TopDownCharacter_C|GetviewportFull (Variables|Default|GetTop%20Down%20Character)))
      (bind _returnvalue (UserInterface|CreateWidget "/Game/UI/Widgets/W_Poster2.W_Poster2_C" 0 self))
      (Variables|/Game/TopDownBP/Blueprints/TopDownCharacter.TopDownCharacter_C|SetwidgeRef (Variables|Default|GetTop%20Down%20Character) _returnvalue)
      (UserInterface|Viewport|AddtoViewport _returnvalue 0)
      (Variables|/Game/TopDownBP/Blueprints/TopDownCharacter.TopDownCharacter_C|SetviewportFull (Variables|Default|GetTop%20Down%20Character) true))))

(fn ConstructionScript)