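; BP_PasswordScreen is an interactable password-locked PC that leads to an email screen.
; When the player character enters or is already inside its sphere while moving to it as the targeted interactable, it opens W_Password with a reference to itself.
; CheckPassword compares the input to the stored password and returns the result.
; A match fires CorrectPassword, which shows W_Emails with the email content and changes the character's objective.
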(event OnComponentBeginOverlap(Sphere)
  (params (OverlappedComponent :type Primitive%20Component%20Object%20Reference) (OtherActor :type Actor%20Object%20Reference) (OtherComp :type Primitive%20Component%20Object%20Reference) (OtherBodyIndex :type Integer) (bFromSweep :type Boolean) (SweepResult :type Hit%20Result%20Structure%20%28by%20ref%29))
  (bind _astop_down_character (Utilities|Casting|CastToTopDownCharacter OtherActor))
  (if (and (Variables|/Game/TopDownBP/Blueprints/TopDownController.TopDownController_C|GetMovingToInteractable (.AsTop%20Down%20Controller (Utilities|Casting|CastToTopDownController (Pawn|GetController _astop_down_character)))) (== (Variables|/Game/TopDownBP/Blueprints/TopDownController.TopDownController_C|GetInteractable (.AsTop%20Down%20Controller (Utilities|Casting|CastToTopDownController (Pawn|GetController _astop_down_character)))) self))
    (Variables|/Game/TopDownBP/Blueprints/TopDownController.TopDownController_C|SetMovingToInteractable (.AsTop%20Down%20Controller (Utilities|Casting|CastToTopDownController (Pawn|GetController _astop_down_character))) false)
    (bind _returnvalue (UserInterface|CreateWidget "/Game/UI/Widgets/W_Password.W_Password_C" 0 self))
    (UserInterface|Viewport|AddtoViewport _returnvalue 0)))

(event Custom|PlayerOverlapCheck
  (if (Utilities|Array|ContainsItem (Collision|GetOverlappingActors (Variables|Default|GetSphere) "/Game/TopDownBP/Blueprints/TopDownCharacter.TopDownCharacter_C" :!class /Script/Engine.PrimitiveComponent) (Game|Player|GetPlayerPawn 0))
    (if (and (Variables|/Game/TopDownBP/Blueprints/TopDownController.TopDownController_C|GetMovingToInteractable (.AsTop%20Down%20Controller (Utilities|Casting|CastToTopDownController (Pawn|GetController (stale OnComponentBeginOverlap(Sphere) _astop_down_character))))) (== (Variables|/Game/TopDownBP/Blueprints/TopDownController.TopDownController_C|GetInteractable (.AsTop%20Down%20Controller (Utilities|Casting|CastToTopDownController (Pawn|GetController (stale OnComponentBeginOverlap(Sphere) _astop_down_character))))) self))
      (Variables|/Game/TopDownBP/Blueprints/TopDownController.TopDownController_C|SetMovingToInteractable (.AsTop%20Down%20Controller (Utilities|Casting|CastToTopDownController (Pawn|GetController (stale OnComponentBeginOverlap(Sphere) _astop_down_character)))) false)
      (bind _returnvalue (UserInterface|CreateWidget "/Game/UI/Widgets/W_Password.W_Password_C" 0 self))
      (UserInterface|Viewport|AddtoViewport _returnvalue 0))))

(event Custom|Correct%20Password
  (bind _returnvalue (UserInterface|CreateWidget "/Game/UI/Widgets/W_Emails.W_Emails_C" 0 (Variables|Default|GetEmailContent)))
  (UserInterface|Viewport|AddtoViewport _returnvalue 0)
  (Default|ObjectiveChanger (stale OnComponentBeginOverlap(Sphere) _astop_down_character) 7))

(fn ConstructionScript)

(fn CheckPassword
  (params (InputPassword :type Text))
  (if (Utilities|Enum|Equal(Enum) InputPassword (Variables|Default|GetPassword))
    (CallFunction|CorrectPassword)
    (return true)
    (else
      (return false))))