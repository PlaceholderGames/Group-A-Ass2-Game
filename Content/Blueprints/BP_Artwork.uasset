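; BP_Artwork is an artwork actor that can be destroyed, with consequences for the player's related opportunities.
; Its Destroy event removes the actor and runs OpportunityPassCheck on the player character for each entry in RelatedOps, at a fixed damage tier.
; PlayerOverlapCheck tests whether the player is inside its Sphere and, if so, clears the TopDownController's MovingToInteractable flag.
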(event Custom|PlayerOverlapCheck
  (bind _sphere (Variables|Default|GetSphere))
  (bind _overlappingactors (Collision|GetOverlappingActors _sphere "/Game/TopDownBP/Blueprints/TopDownCharacter.TopDownCharacter_C" :!class /Script/Engine.PrimitiveComponent))
  (if (Utilities|Array|ContainsItem _overlappingactors (.AsTop%20Down%20Character (Utilities|Casting|CastToTopDownCharacter (Game|Player|GetPlayerPawn 0))))
    (bind _output_get (Variables|Default|SetTopDownCharacter (.AsTop%20Down%20Character (Utilities|Casting|CastToTopDownCharacter (Utilities|Array|Get(acopy) _overlappingactors)))))
    (Variables|/Game/TopDownBP/Blueprints/TopDownController.TopDownController_C|SetMovingToInteractable (.AsTop%20Down%20Controller (Utilities|Casting|CastToTopDownController (Pawn|GetController _output_get))) false)))

(event Custom|Destroy
  (Actor|DestroyActor)
  (for _array_element (Variables|Default|GetrelatedOps)
    (Default|OpportunityPassCheck (.AsTop%20Down%20Character (Utilities|Casting|CastToTopDownCharacter (Game|GetPlayerCharacter 0))) _array_element 4)))

(event EventBeginPlay)

(event Collision|EventActorBeginOverlap
  (params (OtherActor :type Actor%20Object%20Reference)))

(event EventTick
  (params (DeltaSeconds :type Float%20%28single-precision%29)))

(fn ConstructionScript)