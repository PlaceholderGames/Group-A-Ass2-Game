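; BP_Plant is an interactable plant tied to the "Kill all the plants with coffee" opportunity.
; Entering its sphere offers that opportunity to the player character and, unless FullOps is returned, flags every plant as having given it.
; Dead hides mesh parts with a transparent material, marks the plant withered and passes the opportunity once all plants are withered.
; Sphere overlap checks and capsule hits clear the controller's MovingToInteractable state.
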(event OnComponentBeginOverlap(Sphere)
  (params (OverlappedComponent :type Primitive%20Component%20Object%20Reference) (OtherActor :type Actor%20Object%20Reference) (OtherComp :type Primitive%20Component%20Object%20Reference) (OtherBodyIndex :type Integer) (bFromSweep :type Boolean) (SweepResult :type Hit%20Result%20Structure%20%28by%20ref%29))
  (bind _astop_down_character (Utilities|Casting|CastToTopDownCharacter OtherActor))
  (if (not (Variables|Default|GetOpportunityGiven))
    (bind _fullops (Default|OpportunityChanger _astop_down_character "" "Kill all the plants with coffee"))
    (if (not _fullops)
      (bind _outactors (Actor|GetAllActorsOfClass "BP_Plant_C"))
      (for _array_element _outactors
        (Variables|BP_Plant_C|SetOpportunityGiven _array_element true)))))

(event OnComponentHit(Capsule)
  (params (HitComponent :type Primitive%20Component%20Object%20Reference) (OtherActor :type Actor%20Object%20Reference) (OtherComp :type Primitive%20Component%20Object%20Reference) (NormalImpulse :type Vector :default "0, 0, 0") (Hit :type Hit%20Result%20Structure%20%28by%20ref%29))
  (bind _returnvalue (Game|GetPlayerController 0))
  (bind _astop_down_controller (Utilities|Casting|CastToTopDownController _returnvalue))
  (Utilities|Casting|CastToTopDownCharacter OtherActor)
  (if (== (Variables|/Game/TopDownBP/Blueprints/TopDownController.TopDownController_C|GetInteractable _astop_down_controller) self)
    (Variables|/Game/TopDownBP/Blueprints/TopDownController.TopDownController_C|SetMovingToInteractable _astop_down_controller false)))

(event Custom|Dead
  (bind _staticmeshcomponent (Variables|Debug|GetStaticMeshComponent))
  (Rendering|Material|SetMaterial _staticmeshcomponent 1 "/Game/Materials/M_Transparent.M_Transparent")
  (Rendering|Material|SetMaterial _staticmeshcomponent 5 "/Game/Materials/M_Transparent.M_Transparent")
  (Rendering|Material|SetMaterial _staticmeshcomponent 6 "/Game/Materials/M_Transparent.M_Transparent")
  (Variables|Default|SetWithered true)
  (Variables|Default|SetOpportunityCheck true)
  (bind _outactors (Actor|GetAllActorsOfClass "BP_Plant_C"))
  (for _array_element _outactors
    (if (not (Variables|BP_Plant_C|GetWithered _array_element))
      (Variables|Default|SetOpportunityCheck false)))
  (if (Variables|Default|GetOpportunityCheck)
    (Default|OpportunityPassCheck (.AsTop%20Down%20Character (Utilities|Casting|CastToTopDownCharacter (Game|Player|GetPlayerPawn 0))) "Kill all the plants with coffee" 1)))

(event Custom|PlayerOverlapCheck
  (bind _sphere (Variables|Default|GetSphere))
  (bind _overlappingactors (Collision|GetOverlappingActors _sphere "/Game/TopDownBP/Blueprints/TopDownCharacter.TopDownCharacter_C" :!class /Script/Engine.PrimitiveComponent))
  (if (Utilities|Array|ContainsItem _overlappingactors (.AsTop%20Down%20Character (Utilities|Casting|CastToTopDownCharacter (Game|Player|GetPlayerPawn 0))))
    (bind _output_get (Variables|Default|SetTopDownCharacter (.AsTop%20Down%20Character (Utilities|Casting|CastToTopDownCharacter (Utilities|Array|Get(acopy) _overlappingactors)))))
    (Variables|/Game/TopDownBP/Blueprints/TopDownController.TopDownController_C|SetMovingToInteractable (.AsTop%20Down%20Controller (Utilities|Casting|CastToTopDownController (Pawn|GetController _output_get))) false)))

(event EventBeginPlay)

(event Collision|EventActorBeginOverlap
  (params (OtherActor :type Actor%20Object%20Reference)))

(event EventTick
  (params (DeltaSeconds :type Float%20%28single-precision%29)))

(fn ConstructionScript)